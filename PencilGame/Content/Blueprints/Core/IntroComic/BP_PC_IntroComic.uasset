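; Player controller for the intro comic that plays a video intro when the level begins.
; BeginPlay clears existing widgets, adds the W_IntroVideo widget to the viewport and starts a media sound component for its audio.
; It switches to UI-only input with a hidden cursor and blocks player input for a fixed delay before re-enabling it.
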(event EventBeginPlay
  (bind _returnvalue (Game|GetPlayerController 0))
  (Utilities|FlowControl|Sequence
    (:then_0
      (Viewport|RemoveAllWidgets))
    (:then_1
      (bind _returnvalue_2 (UserInterface|CreateWidget "/Game/Video/W_IntroVideo.W_IntroVideo_C"))
      (UserInterface|Viewport|AddtoViewport _returnvalue_2 0)
      (CameraShake|Start (Variables|Default|GetMediaSound))
      (Input|DisableInput _returnvalue)
      (Utilities|FlowControl|Delay 22.0)
      (Input|EnableInput _returnvalue))
    (:then_2
      (Input|SetInputModeUIOnly self 0 "DoNotLock")
      (Variables|Default|SetbShowMouseCursor false))))

(event EventTick
  (params (DeltaSeconds :type Float%20%28single-precision%29)))

(fn ConstructionScript)